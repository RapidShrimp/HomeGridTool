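; Portal actor that shows the view out of its linked portal through a viewport-sized render target fed into a dynamic material on its surface.
; Each tick in PostUpdateWork, it moves the linked portal's capture camera to the player camera's transform, mirrored into that portal's space.
; It clips its own capture camera with a plane at the portal face to hide geometry behind it.
; The render target resizes whenever the viewport size changes.
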(event `self.ReceiveBeginPlay`
  (bind (_returnvalue_x _returnvalue_y) (`KismetMathLibrary.BreakVector2D` (`WidgetLayoutLibrary.GetViewportSize`)))
  (`self.SetTickGroup` "TG_PostUpdateWork")
  (bind _returnvalue (`KismetMaterialLibrary.CreateDynamicMaterialInstance` "/Game/Core/PortalMaterial.PortalMaterial"))
  (bind _output_get (set `self.PortalMaterial` _returnvalue))
  (`PrimitiveComponent.SetMaterial` (`self.Portal`) 0 _output_get)
  (bind _returnvalue_2 (`KismetRenderingLibrary.CreateRenderTarget2D` (`KismetMathLibrary.FTrunc` _returnvalue_x) (`KismetMathLibrary.FTrunc` _returnvalue_y)))
  (bind _output_get_2 (set `self.PortalRenderTarget` _returnvalue_2))
  (`MaterialInstanceDynamic.SetTextureParameterValue` (`self.PortalMaterial`) "PortalRT" _output_get_2)
  (set `SceneCaptureComponent2D.TextureTarget` (`self.PortalRenderTarget`) (`/Game/Core/BP_Portal_OLD.PortalCamera` (`self.LinkedPortal`)))
  (`self.SetPlanarClipping`))

(event `self.ReceiveTick`
  (params (DeltaSeconds :type "Float (single-precision)"))
  (`self.UpdateSceneCapture`)
  (`self.CheckViewSize`))

(fn `CheckViewSize`
  (bind _portalrendertarget (`self.PortalRenderTarget`))
  (bind (_x _y) (`KismetMathLibrary.BreakVector2D` (`WidgetLayoutLibrary.GetViewportSize`)))
  (bind (_x_2 _y_2) (`KismetMathLibrary.BreakVector2D` (`WidgetLayoutLibrary.GetViewportSize`)))
  (if (not (and (== _x (`TextureRenderTarget2D.SizeX` _portalrendertarget)) (== _y (`TextureRenderTarget2D.SizeY` _portalrendertarget))))
    (`KismetSystemLibrary.LogString` "Rezsizing Viewport")
    (`KismetRenderingLibrary.ResizeRenderTarget2D` (`self.PortalRenderTarget`) (`KismetMathLibrary.FTrunc` _x_2) (`KismetMathLibrary.FTrunc` _y_2))))

(fn `GetUpdatedLocation`
  (returns (ReturnValue :type "Vector Structure"))
  (bind _transformcomponent (`PlayerCameraManager.TransformComponent` (`GameplayStatics.GetPlayerCameraManager` 0))
    (:`then`
      (bind _linkedportal (`self.LinkedPortal`)
        (:`then`
          (return (`KismetMathLibrary.TransformLocation` (`self.GetTransform` _linkedportal) (`KismetMathLibrary.InverseTransformLocation` (`KismetMathLibrary.MakeTransform` (.location (`self.GetTransform`)) (.rotation (`self.GetTransform`)) (`KismetMathLibrary.MakeVector` (* (.x (.scale (`self.GetTransform`))) -1.0) (* (.y (.scale (`self.GetTransform`))) -1.0) (.z (.scale (`self.GetTransform`))))) (`SceneComponent.K2_GetComponentLocation` _transformcomponent)))))
        (:`else`
          (`KismetSystemLibrary.LogString` "No Linked Portal Found")
          (return (0.0 0.0 0.0)))))
    (:`else`
      (`KismetSystemLibrary.LogString` "No Camera Transform Component")
      (return (0.0 0.0 0.0)))))

(fn `GetUpdatedRotation`
  (returns (ReturnValue :type "Rotator Structure"))
  (bind _returnvalue (`self.GetTransform`))
  (bind _returnvalue_2 (`self.GetTransform` (`self.LinkedPortal`)))
  (bind (_x _y _z) (`KismetMathLibrary.BreakRotIntoAxes` (`SceneComponent.K2_GetComponentRotation` (`PlayerCameraManager.TransformComponent` (`GameplayStatics.GetPlayerCameraManager` 0)))))
  (return (`KismetMathLibrary.MakeRotationFromAxes` (`KismetMathLibrary.TransformDirection` _returnvalue_2 (`KismetMathLibrary.MirrorVectorByNormal` (`KismetMathLibrary.MirrorVectorByNormal` (`KismetMathLibrary.InverseTransformDirection` _returnvalue _x) (1.0 0.0 0.0)) (0.0 1.0 0.0))) (`KismetMathLibrary.TransformDirection` _returnvalue_2 (`KismetMathLibrary.MirrorVectorByNormal` (`KismetMathLibrary.MirrorVectorByNormal` (`KismetMathLibrary.InverseTransformDirection` _returnvalue _y) (1.0 0.0 0.0)) (0.0 1.0 0.0))) (`KismetMathLibrary.TransformDirection` _returnvalue_2 (`KismetMathLibrary.MirrorVectorByNormal` (`KismetMathLibrary.MirrorVectorByNormal` (`KismetMathLibrary.InverseTransformDirection` _returnvalue _z) (1.0 0.0 0.0)) (0.0 1.0 0.0))))))

(fn `SetPlanarClipping`
  (bind _portalcamera (`self.PortalCamera`))
  (`/Engine/EditorBlueprintResources/StandardMacros.IsValid` (`self.LinkedPortal`)
    (:`Is Valid`
      (set `SceneCaptureComponent2D.bEnableClipPlane` true _portalcamera)
      (set `SceneCaptureComponent2D.ClipPlaneBase` (+ (`SceneComponent.K2_GetComponentLocation` (`self.Portal`)) (* (`SceneComponent.GetForwardVector` (`self.ForwardDir`)) -3.0)) _portalcamera)
      (set `SceneCaptureComponent2D.ClipPlaneNormal` (`SceneComponent.GetForwardVector` (`self.ForwardDir`)) _portalcamera))))

(fn `UpdateSceneCapture`
  (bind _linkedportal (`self.LinkedPortal`)
    (:`then`
      (`SceneComponent.K2_SetWorldLocationAndRotation` (`/Game/Core/BP_Portal_OLD.PortalCamera` _linkedportal) (`self.GetUpdatedLocation`) (`self.GetUpdatedRotation`) false false))
    (:`else`)))

(fn `UserConstructionScript`)