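; Level manager component for level generation that restores Level_Chunk actors and places doors where chunks connect.
; On BeginPlay it calls SpawnSaved on every Level_Chunk in the world.
; SpawnDoors gathers open door locations from the given chunks and spawns a BP_Door wherever one matches an earlier location, exactly or within a small distance.
; Each door takes the socket's rotation with a quarter-turn yaw offset.
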(event `self.ReceiveBeginPlay`
  (bind _outactors (`GameplayStatics.GetAllActorsOfClass` "/Game/Core/LevelGen/Level_Chunk.Level_Chunk_C"))
  (for _array_element _outactors
    (`/Game/Core/LevelGen/Level_Chunk.SpawnSaved` _array_element)))

(fn `SpawnDoorAtTransform`
  (params (InTransform :type "Transform Structure"))
  (`|SpawnActorFromClass` "/Game/Core/LevelGen/BP_Door.BP_Door_C" InTransform "Undefined" "MultiplyWithRoot" null null))

(fn `SpawnDoors`
  (params (Levels :type "Array of /Game/Core/LevelGen/Level_Chunk Object Reference"))
  (locals (WorldLocations :type "Array of IntVector Structure"))
  (`KismetArrayLibrary.Array_Clear` (`local.WorldLocations`))
  (for _array_element Levels
    (bind (_doors _opendoorlocations) (`/Game/Core/LevelGen/Level_Chunk.GetDoorLocations` _array_element))
    (for (_array_element_2 _array_index) _opendoorlocations
      (`|ExecutionSequence`
        (:`then_0`
          (if (`KismetArrayLibrary.Array_Contains` (`local.WorldLocations`) _array_element_2)
            (bind _returnvalue (`KismetMathLibrary.MakeRotator` (.roll (`SceneComponent.K2_GetComponentRotation` (`|GetArrayItem` _doors _array_index))) (.pitch (`SceneComponent.K2_GetComponentRotation` (`|GetArrayItem` _doors _array_index))) (+ (.yaw (`SceneComponent.K2_GetComponentRotation` (`|GetArrayItem` _doors _array_index))) 90.0)))
            ;[1 1 1] Found Item
            (`self.SpawnDoorAtTransform` (`KismetMathLibrary.MakeTransform` (`KismetMathLibrary.Conv_IntVectorToVector` _array_element_2) _returnvalue))
            (else
              ;[1 1 1] Distance Check
              (for _array_element_3 (`local.WorldLocations`)
                (bind _returnvalue_2 (`KismetMathLibrary.Conv_IntVectorToVector` _array_element_2))
                (if (< (`KismetMathLibrary.Vector_Distance` (`KismetMathLibrary.Conv_IntVectorToVector` _array_element_3) _returnvalue_2) 5.0)
                  (`self.SpawnDoorAtTransform` (`KismetMathLibrary.MakeTransform` _returnvalue_2 _returnvalue)))))))
        (:`then_1`
          (`KismetArrayLibrary.Array_Add` (`local.WorldLocations`) _array_element_2)))))
  (return))