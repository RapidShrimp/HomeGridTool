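; Level builder behind an editor tool for assembling levels from a tree of connected Level_Chunk rooms.
; It tracks placed chunks, adds children to the selected one by direction, and box-traces open sides to report spawn options.
; Edits to room size, doors and offsets write into the chunk's layout struct and rebuild its visuals.
; A spawned CreateWidgetActor follows the selection and is destroyed on tool shutdown.
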(event `Init`
  (params (EditorWidget :type "/Game/Core/LevelGen/EditorUtlity/EUW_BuilderTool Object Reference"))
  (set `self.BuilderEditorWidget` EditorWidget)
  (`self.CreateWidgetViewer`))

(event `FindAllRooms`
  (`KismetArrayLibrary.Array_Clear` (`self.LevelChunks`))
  (bind _outactors (`GameplayStatics.GetAllActorsOfClass` "/Game/Core/LevelGen/Level_Chunk.Level_Chunk_C"))
  (bind _output_get (set `self.LevelChunks` _outactors))
  (if (`KismetArrayLibrary.Array_IsEmpty` _output_get)
    (bind _returnvalue (`|SpawnActorFromClass` "/Game/Core/LevelGen/Level_Chunk.Level_Chunk_C" (`KismetMathLibrary.MakeTransform` (0.0 0.0 200.0)) "AdjustIfPossibleButAlwaysSpawn" "MultiplyWithRoot" null null))
    (`self.SetRootChunk` _returnvalue)
    (`self.AddLevelChunk` _returnvalue)
    (`self.SelectChunk` _returnvalue)
    (else
      (`self.SetRootChunk` (`|GetArrayItem` _output_get)))))

(event `CreateWidgetViewer`
  (`/Engine/EditorBlueprintResources/StandardMacros.IsValid` (`self.CreateWidgetActor`)
    (:`Is Not Valid`
      (bind _returnvalue (`|SpawnActorFromClass` "/Game/Core/LevelGen/EditorUtlity/Builder/CreateWidgetActor.CreateWidgetActor_C" (`KismetMathLibrary.MakeTransform` (0.0 0.0 0.0)) "AlwaysSpawn" "MultiplyWithRoot" null null))
      (bind _output_get (set `self.CreateWidgetActor` _returnvalue))
      (set `/Game/Core/LevelGen/EditorUtlity/Builder/CreateWidgetActor.Builder` self _output_get))))

(fn `AddLevelChunk`
  (params (ChunkToAdd :type "/Game/Core/LevelGen/Level_Chunk Object Reference"))
  (returns (Success :type Boolean))
  (`/Engine/EditorBlueprintResources/StandardMacros.IsValid` ChunkToAdd
    (:`Is Valid`
      (`KismetArrayLibrary.Array_AddUnique` (`self.LevelChunks`) ChunkToAdd)
      (`self.SelectChunk` ChunkToAdd)
      (return true))
    (:`Is Not Valid`
      (return false))))

(fn `CheckCanSpawnInDirection`
  (params (Direction :type "/Game/Core/LevelGen/Enums/E_DoorDirection Enum" :default "NewEnumerator0"))
  (returns (CanPlace :type Boolean))
  (bind _selectedchunk (`self.SelectedChunk`))
  (bind _returnvalue (`SceneComponent.K2_GetComponentLocation` (select `/Game/Core/LevelGen/Enums/E_DoorDirection` Direction :`NewEnumerator0` (`/Game/Core/LevelGen/Level_Chunk.Entry` _selectedchunk) :`NewEnumerator1` (`/Game/Core/LevelGen/Level_Chunk.Forward` _selectedchunk) :`NewEnumerator2` (`/Game/Core/LevelGen/Level_Chunk.Left` _selectedchunk) :`NewEnumerator3` (`/Game/Core/LevelGen/Level_Chunk.Right` _selectedchunk))))
  (bind (_outhit _returnvalue_2) (`KismetSystemLibrary.BoxTraceSingle` _returnvalue (+ _returnvalue (* (select `/Game/Core/LevelGen/Enums/E_DoorDirection` "NewEnumerator0" :!type "Vector Structure") 300.0)) (150.0 150.0 150.0) (struct) "TraceTypeQuery1" false (`|MakeArray` (`self.CreateWidgetActor`) (`self.SelectedChunk`) :!type "Actor Object Reference") "ForDuration"))
  (if _returnvalue_2
    (cast `/Game/Core/LevelGen/Level_Chunk` (`.HitActor` (`GameplayStatics.BreakHitResult` _outhit))
      (:`then`
        (return false))
      (:`CastFailed`
        (return true)))
    (else
      (return false))))

(fn `ChunkUpdated`
  (`/Game/Core/LevelGen/EditorUtlity/Builder/CreateWidgetActor.OnNewChunkSelected` (`self.CreateWidgetActor`) (`self.SelectedChunk`))
  (`/Game/Core/LevelGen/Level_Chunk.CreateRoomVisuals` (`self.SelectedChunk`)))

(fn `CreateNewChunk`
  (params (RoomDirection :type "/Game/Core/LevelGen/Enums/E_DoorDirection Enum" :default "NewEnumerator0") (Defaults :type "/Game/Core/LevelGen/Tables/Structs/S_RoomData Structure"))
  (bind _selectedchunk (`self.SelectedChunk`))
  (`/Engine/EditorBlueprintResources/StandardMacros.IsValid` _selectedchunk
    (:`Is Valid`
      (bind _outchunk (`/Game/Core/LevelGen/Level_Chunk.AddChildChunk` _selectedchunk (`self.SelectedChunk`) RoomDirection Defaults))
      (`self.AddLevelChunk` _outchunk)
      (`self.ValidateChunks`))
    (:`Is Not Valid`
      (`KismetSystemLibrary.LogString` "No Selected Chunk"))))

(fn `Get Saved Selected Chunk`
  (returns (SelectedChunk :type "/Game/Core/LevelGen/Level_Chunk Object Reference") (ReturnValue :type Boolean))
  (bind _selectedchunk (`self.SelectedChunk`))
  (return _selectedchunk (`KismetSystemLibrary.IsValid` _selectedchunk)))

(fn `GetRoomInDirection`
  (params (Direction :type "/Game/Core/LevelGen/Enums/E_DoorDirection Enum" :default "NewEnumerator0"))
  (returns (HasRoom :type Boolean) (RoomRef :type "/Game/Core/LevelGen/Level_Chunk Object Reference"))
  (bind _selectedchunk (`self.SelectedChunk`)
    (:`then`
      (bind _childchunks (`/Game/Core/LevelGen/Level_Chunk.ChildChunks` _selectedchunk))
      (if (`BlueprintMapLibrary.Map_Contains` _childchunks Direction)
        (bind (_value _returnvalue) (`BlueprintMapLibrary.Map_Find` _childchunks Direction))
        (return _returnvalue _value)
        (else
          (return false null))))
    (:`else`
      (return false null))))

(fn `GetSpawnDirectionData`
  (returns (Results :type "Map of /Game/Core/LevelGen/Enums/E_DoorDirection Enum to Boolean"))
  (locals (Directions :type "Map of /Game/Core/LevelGen/Enums/E_DoorDirection Enum to Boolean"))
  (`|ExecutionSequence`
    (:`then_0`
      (if (not (`BlueprintMapLibrary.Map_Contains` (`/Game/Core/LevelGen/Level_Chunk.ChildChunks` (`self.SelectedChunk`)) "NewEnumerator1"))
        (bind _canplace (`self.CheckCanSpawnInDirection` "NewEnumerator1"))
        (`BlueprintMapLibrary.Map_Add` (`local.Directions`) "NewEnumerator1" _canplace)))
    (:`then_1`
      (if (not (`BlueprintMapLibrary.Map_Contains` (`/Game/Core/LevelGen/Level_Chunk.ChildChunks` (`self.SelectedChunk`)) "NewEnumerator2"))
        (bind _canplace_2 (`self.CheckCanSpawnInDirection` "NewEnumerator2"))
        (`BlueprintMapLibrary.Map_Add` (`local.Directions`) "NewEnumerator2" _canplace_2)))
    (:`then_2`
      (if (not (`BlueprintMapLibrary.Map_Contains` (`/Game/Core/LevelGen/Level_Chunk.ChildChunks` (`self.SelectedChunk`)) "NewEnumerator3"))
        (bind _canplace_3 (`self.CheckCanSpawnInDirection` "NewEnumerator3"))
        (`BlueprintMapLibrary.Map_Add` (`local.Directions`) "NewEnumerator3" _canplace_3)))
    (:`then_3`
      (`KismetSystemLibrary.LogString` "Ran Here")
      (return (`local.Directions`)))))

(fn `OnToolShutdown`
  (`self.K2_DestroyActor` (`self.CreateWidgetActor`))
  (set `self.CreateWidgetActor` null))

(fn `RemoveLevelChunk`
  (params (ChunkToRemove :type "/Game/Core/LevelGen/Level_Chunk Object Reference") (`Remove Children` :type Boolean))
  (returns (Success :type Boolean))
  (`/Engine/EditorBlueprintResources/StandardMacros.IsValid` ChunkToRemove
    (:`Is Valid`
      (if `Remove Children`
        (`/Game/Core/LevelGen/Level_Chunk.RemoveChildrenRecursive` (`self.SelectedChunk`))
        (`self.ValidateChunks`)
        (return true)
        (else
          (bind _returnvalue (`KismetArrayLibrary.Array_RemoveItem` (`self.LevelChunks`) ChunkToRemove))
          (return _returnvalue))))
    (:`Is Not Valid`
      (return false))))

(fn `SelectChunk`
  (params (`Selected Chunk` :type "/Game/Core/LevelGen/Level_Chunk Object Reference"))
  (bind _createwidgetactor (`self.CreateWidgetActor`))
  (`/Engine/EditorBlueprintResources/StandardMacros.IsValid` `Selected Chunk`
    (:`Is Valid`
      (set `self.SelectedChunk` `Selected Chunk`)
      (`self.K2_SetActorLocation` _createwidgetactor (`self.K2_GetActorLocation` `Selected Chunk`) false true)
      (`/Game/Core/LevelGen/EditorUtlity/Builder/CreateWidgetActor.OnNewChunkSelected` _createwidgetactor `Selected Chunk`)
      (`self.ValidateChunks`))))

(fn `SetRootChunk`
  (params (`First Chunk` :type "/Game/Core/LevelGen/Level_Chunk Object Reference") (`Override All` :type Boolean))
  (`/Engine/EditorBlueprintResources/StandardMacros.IsValid` `First Chunk`
    (:`Is Valid`
      (if (or (and `Override All` (`KismetSystemLibrary.IsValid` (`self.FirstChunk`))) (not (`KismetSystemLibrary.IsValid` (`self.FirstChunk`))))
        (set `self.FirstChunk` `First Chunk`)))
    (:`Is Not Valid`
      (`KismetSystemLibrary.LogString` "No Chunk Avaliable"))))

(fn `Update Custom Room Size`
  (params (CustomRoomScale :type "Vector2D Structure"))
  (bind _selectedchunk (`self.SelectedChunk`))
  (bind _structout (setmembers `/Game/Core/LevelGen/Tables/Structs/S_RoomData` :`StructRef` (`/Game/Core/LevelGen/Level_Chunk.Room Layout` _selectedchunk) :`CustomRoomScale` CustomRoomScale))
  (set `/Game/Core/LevelGen/Level_Chunk.Room Layout` _structout _selectedchunk)
  (`self.ChunkUpdated`))

(fn `Update Door Offsets`
  (params (Offsets :type "Map of /Game/Core/LevelGen/Enums/E_DoorDirection Enum to Vector2D Structure"))
  (bind _selectedchunk (`self.SelectedChunk`))
  (bind _structout (setmembers `/Game/Core/LevelGen/Tables/Structs/S_RoomData` :`StructRef` (`/Game/Core/LevelGen/Level_Chunk.Room Layout` _selectedchunk) :`Offsets` Offsets))
  (set `/Game/Core/LevelGen/Level_Chunk.Room Layout` _structout _selectedchunk)
  (`self.ChunkUpdated`))

(fn `Update Doors`
  (params (`Forward Door` :type Boolean) (`Left Door` :type Boolean) (`Right Door` :type Boolean))
  (bind _selectedchunk (`self.SelectedChunk`))
  (bind _structout (setmembers `/Game/Core/LevelGen/Tables/Structs/S_RoomData` :`StructRef` (`/Game/Core/LevelGen/Level_Chunk.Room Layout` _selectedchunk) :`Forward Door` `Forward Door` :`Left Door` `Left Door` :`Right Door` `Right Door`))
  (set `/Game/Core/LevelGen/Level_Chunk.Room Layout` _structout _selectedchunk)
  (`self.ChunkUpdated`))

(fn `Update Room Size`
  (params (`Room Scale` :type "/Game/Core/LevelGen/Enums/E_RoomSize Enum" :default "NewEnumerator0"))
  (bind _selectedchunk (`self.SelectedChunk`))
  (bind _structout (setmembers `/Game/Core/LevelGen/Tables/Structs/S_RoomData` :`StructRef` (`/Game/Core/LevelGen/Level_Chunk.Room Layout` _selectedchunk) :`Room Scale` `Room Scale`))
  (set `/Game/Core/LevelGen/Level_Chunk.Room Layout` _structout _selectedchunk)
  (`self.ChunkUpdated`))

(fn `UserConstructionScript`)

(fn `ValidateChunks`
  (bind _firstchunk (`self.FirstChunk`)
    (:`then`
      (`/Game/Core/LevelGen/Level_Chunk.ValidateChildren` _firstchunk)
      (`self.ChunkUpdated`))
    (:`else`)))